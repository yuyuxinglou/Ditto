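; Base pickup actor that gives the player an inventory item through the Interactive input.
; Player-tagged overlap adds a named WB_PickupItem entry to the character's pickup widget, enables input and opens a gate.
; Pressing Interactive through that gate adds the item, count and level via the player controller, then destroys the actor.
; End overlap removes the entry and hides an empty list, but neither closes the gate nor disables input.
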(event `GiveItem`
  (`RPGPlayerControllerBase.AddInventoryItem` (`/Game/Blueprints/BP_RPGFunctionLibrary.Get Player Controller BP`) (`self.ItemType`) (`self.Item Count`) (`self.Item Level`) true))

(event `InputAction|Interactive`
  (params (Key :type "Key Structure"))
  (:`Pressed`
    (`/Engine/EditorBlueprintResources/StandardMacros.Gate` true :!label _label
      (:`Exit`
        (`self.GiveItem`)
        (`self.K2_DestroyActor`)))))

(event `self.CollectCollsion.OnComponentBeginOverlap`
  (params (OverlappedComponent :type "PrimitiveComponent Object Reference") (OtherActor :type "Actor Object Reference") (OtherComp :type "PrimitiveComponent Object Reference") (OtherBodyIndex :type Integer) (bFromSweep :type Boolean) (SweepResult :type "HitResult Structure (by ref)"))
  (if (`self.ActorHasTag` OtherActor "Player")
    (bind _returnvalue (`|CreateWidget` "/Game/Blueprints/WidgetBP/Inventory/WB_PickupItem.WB_PickupItem_C"))
    (bind _output_get (set `self.TempItem` _returnvalue))
    (`TextBlock.SetText` (`/Game/Blueprints/WidgetBP/Inventory/WB_PickupItem.PickupItemText` _output_get) (`RPGItem.ItemName` (`self.ItemType`)))
    (bind _asbp_player_character_1 (cast `/Game/Blueprints/BP_PlayerCharacter1` OtherActor))
    (bind _output_get_2 (set `self.As BP Player Character` _asbp_player_character_1))
    (bind _itempickup (`/Game/Blueprints/BP_PlayerCharacter1.ItemPickup` _output_get_2))
    (`SceneComponent.SetVisibility` _itempickup true false)
    (bind _aswb_pickup (cast `/Game/Blueprints/WidgetBP/Inventory/WB_Pickup` (`WidgetComponent.GetWidget` _itempickup)))
    (bind _output_get_3 (set `self.As WB Pickup` _aswb_pickup))
    (`PanelWidget.AddChild` (`/Game/Blueprints/WidgetBP/Inventory/WB_Pickup.PickItemBox` _output_get_3) (`self.TempItem`))
    (`self.EnableInput` (`GameplayStatics.GetPlayerController` 0))
    (goto _label :!via `Open`)))

(event `self.CollectCollsion.OnComponentEndOverlap`
  (params (OverlappedComponent :type "PrimitiveComponent Object Reference") (OtherActor :type "Actor Object Reference") (OtherComp :type "PrimitiveComponent Object Reference") (OtherBodyIndex :type Integer))
  (bind _pickitembox (`/Game/Blueprints/WidgetBP/Inventory/WB_Pickup.PickItemBox` (`self.As WB Pickup`)))
  (if (`self.ActorHasTag` OtherActor "Player")
    (`PanelWidget.RemoveChild` _pickitembox (`self.TempItem`))
    (if (not (`PanelWidget.HasAnyChildren` _pickitembox))
      (`SceneComponent.SetVisibility` (`/Game/Blueprints/BP_PlayerCharacter1.ItemPickup` (`self.As BP Player Character`)) false false))))

(fn `UserConstructionScript`)
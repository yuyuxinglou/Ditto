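; Game mode Blueprint that sets up the intro cutscene and a 2D sound when play begins.
; BeginPlay calls a custom event that creates a level sequence player for the first intro shot, then spawns the sound.
; The player's validity check leads to nothing, and no Play call follows.
; Nodes for a skippable cutscene on the player controller and for restarting the player are disconnected and never run.
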(event `self.ReceiveBeginPlay`
  (`self.PlayDefaultIntroCutscence`)
  (`GameplayStatics.SpawnSound2D` null 1.0 1.0 0.0 null))

(event `PlayDefaultIntroCutscence`
  (bind _outactor (`LevelSequencePlayer.CreateLevelSequencePlayer` "/Game/Sequences/Intro/shots/SQ_Intro_Shot_001.SQ_Intro_Shot_001"))
  (if (`KismetSystemLibrary.IsValid` _outactor)
    _))

(fn `UserConstructionScript`)